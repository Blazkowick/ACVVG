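; GameControllerBP is a game controller that sets up the HUD and music and applies the effects of collected pickups.
; On BeginPlay it creates and stores the BpHUD widget, caches the bpPlayer pawn and plays a 2D song.
; OnPickUp casts the pickup to tell its type: hearts add unclamped health to a player below a threshold, while coins increment the RingsCollected counter.
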(event EventBeginPlay
  (bind _returnvalue (UserInterface|CreateWidget "/Game/Blueprints/Player/Components/bpHUD.bpHUD_C" (Game|GetPlayerController 0)))
  (bind _output_get (Variables|Default|SetHUDReference _returnvalue))
  (UserInterface|Viewport|AddtoViewport _output_get -20)
  (bind _asbp_player (Utilities|Casting|CastTobpPlayer (Game|Player|GetPlayerPawn 0)))
  (Variables|Default|SetPlayerBP _asbp_player)
  (Audio|PlaySound2D "/Game/Sounds/Musica/Cancion01.Cancion01" 1.5 1.0 0.0 0 0))

(fn ConstructionScript)

(fn OnPickUp
  (params (PickUpType :type Bp%20Pick%20Up%20Base%20Object%20Reference))
  (bind _playerbp (Variables|Default|GetPlayerBP))
  (Utilities|Casting|CastToBP_PickUp_Heart PickUpType
    (:then
      (if (< (Variables|/Game/Blueprints/Player/bpPlayer.bpPlayer_C|GetHealth (Variables|Default|GetPlayerBP)) 99.0)
        (Variables|/Game/Blueprints/Player/bpPlayer.bpPlayer_C|SetHealth _playerbp (+ 2e+01 (Variables|/Game/Blueprints/Player/bpPlayer.bpPlayer_C|GetHealth _playerbp)))))
    (:CastFailed
      (Utilities|Casting|CastToBP_PickUp_Coin PickUpType)
      (Variables|Default|SetRingsCollected (+ (Variables|Default|GetRingsCollected) 1))
      (Utilities|Casting|CastTobpPlayer (Game|GetPlayerCharacter 0)))))