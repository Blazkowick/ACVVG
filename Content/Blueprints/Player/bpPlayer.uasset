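; Player character for a 2D flipbook side-scroller, with running, ladder climbing, air jumps and wall jumps.
; Tick flips the sprite, plays footsteps and selects flipbooks through a priority-based state function, with attack inputs unwired.
; A line trace chooses wall or air jump, while dust actors and timeline squash accent movement.
; It also handles HUD creation, mushroom scaling, death and level-reload respawn; damage is stubbed off by a constant condition.
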(event Custom|JumpFX
  ;[1 1 1] Efectos especiales
  (Game|SpawnActorfromClass "/Game/Blueprints/Actors_FX/bp_Dust.bp_Dust_C" (Transformation|GetWorldTransform (Variables|Default|GetDust)) "AlwaysSpawn" 0 0)
  (bind _squash (Timeline|Timeline_0 PlayFromStart)
    (:Update
      (Transformation|SetActorScale3D (Math|Vector|Lerp(Vector) (Variables|Default|GetCurrentScale) "3.000000,1.000000,0.500000" _squash)))))

(event Custom|LandFX
  ;[1 1 1] Efectos especiales
  (Game|SpawnActorfromClass "/Game/Blueprints/Actors_FX/bp_Dust.bp_Dust_C" (Transformation|GetWorldTransform (Variables|Default|GetDust)) "AlwaysSpawn" 0 0)
  (bind _squash (Timeline|Timeline_1 PlayFromStart)
    (:Update
      (Transformation|SetActorScale3D (Math|Vector|Lerp(Vector) (Variables|Default|GetCurrentScale) "6.000000,1.000000,0.100000" _squash)))))

(event Custom|WallJump
  (bind _returnvalue (Transformation|GetActorForwardVector))
  ;[1 1 1] Movimiento/Salto
  ;;[1 1 1] Salto en paredes
  (bind (_outhit _returnvalue_2) (Collision|LineTraceByChannel (- (Transformation|GetActorLocation) (* _returnvalue (+ (Components|Capsule|GetScaledCapsuleRadius (Variables|Collision|GetCapsuleComponent)) 2.0))) (+ (Transformation|GetActorLocation) (* _returnvalue (+ (Components|Capsule|GetScaledCapsuleRadius (Variables|Collision|GetCapsuleComponent)) 2.0))) "TraceTypeQuery1" true 0 "None"))
  (if _returnvalue_2
    (Character|LaunchCharacter (Math|Vector|MakeVector (* (Math|Float|Sign(Float) (- (.x (Transformation|GetActorLocation)) (.x (.Location (Collision|BreakHitResult _outhit))))) 1.5e+02) 0.0 (Variables|/Script/Engine.CharacterMovementComponent|GetJumpZVelocity (Variables|Character|GetCharacterMovement))) true true)
    (CallFunction|WallJumpFX)
    (elif (< (Variables|Default|GetJumpCurrentCount) (Variables|Default|GetJumpMaxCount))
      (Character|Jump)
      (CallFunction|AirJumpFx))))

(event Custom|WallJumpFX
  ;[1 1 1] Efectos especiales
  (Game|SpawnActorfromClass "/Game/Blueprints/Actors_FX/bp_DustWall.bp_DustWall_C" (Transformation|GetWorldTransform (Variables|Default|GetSprite)) "AlwaysSpawn" 0 0)
  (bind _squash (Timeline|Timeline_4 PlayFromStart)
    (:Update
      (Transformation|SetActorScale3D (Math|Vector|Lerp(Vector) (Variables|Default|GetCurrentScale) "6.000000,1.000000,0.500000" _squash)))))

(event Custom|Respawn
  ;[1 1 1] INICIO DE JUEGO
  (Default|FadeOut (Variables|Default|GetFade_ref))
  (Utilities|FlowControl|Delay 1.0)
  (bind _returnvalue (Game|GetCurrentLevelName true))
  (Game|OpenLevel(byName) (Utilities|String|StringToName _returnvalue)))

(event Custom|Jump%20Event
  (bind _charactermovement (Variables|Character|GetCharacterMovement))
  (bind _returnvalue (AI|Components|NavMovement|IsFalling _charactermovement))
  ;[1 1 1] Movimiento/Salto
  ;;[1 1 1] Saltando
  (if _returnvalue
    (CallFunction|WallJump)
    (Audio|PlaySound2D "/Game/Sounds/Player/Airjump_Cue.Airjump_Cue" 1.0 1.5 0.0 0 0)
    (else
      (Character|Jump)
      (Audio|PlaySound2D "/Game/Sounds/Player/Airjump_Cue.Airjump_Cue" 1.0 1.5 0.0 0 0)
      (if _returnvalue
        (CallFunction|JumpFX)))))

(event Custom|UpdateAnimation
  ;[1 1 1] Animation Handler
  ;;[1 1 1] Gestion de animaciones
  (Variables|Default|SetbIsMoving (> (Math|Vector|VectorLength (Transformation|GetVelocity)) 0.0))
  (bind _outputfb (CallFunction|AnimationStateMachine false false (Variables|Default|GetbIsClimbing) false false false false (AI|Components|NavMovement|IsFalling (Variables|Character|GetCharacterMovement)) (Variables|Default|GetbIsMoving) (Variables|Default|GetbIsIdleCalm) (Variables|Default|GetbIsAlive)))
  (Sprite|SetFlipbook (Variables|Default|GetSprite) _outputfb))

(event Custom|AirJumpFx
  ;[1 1 1] Efectos especiales
  (Game|SpawnActorfromClass "/Game/Blueprints/Actors_FX/bp_DustAir.bp_DustAir_C" (Transformation|GetWorldTransform (Variables|Default|GetSprite)) "AlwaysSpawn" 0 0))

(event Custom|ClimbingEnd
  ;[1 1 1] Movimiento/Salto
  ;;[1 1 1] Escalar (escaleras)
  (Pawn|Components|CharacterMovement|SetMovementMode (Variables|Character|GetCharacterMovement) "MOVE_Walking" 0)
  (Variables|Default|SetbIsClimbing false)
  (Variables|Default|SetbCanMoveRight true)
  (Components|Timeline|SetPlayRate (Variables|Default|GetSprite) 1.0))

(event Custom|SetDir
  (params (DeltaSeconds :type Float%20%28single-precision%29))
  ;[1 1 1] Animation Handler
  ;;[1 1 1] Rotación de animaciones
  (Math|Float|CompareFloat (.X (Math|Vector|BreakVector (Variables|/Script/Engine.MovementComponent|GetVelocity (Variables|Character|GetCharacterMovement)))) 0.0
    (:>
      (Variables|Default|SetMright true))
    (:<
      (Variables|Default|SetMleft true))))

(event Game|Damage|EventAnyDamage
  (params (Damage :type Float%20%28single-precision%29) (DamageType :type Damage%20Type%20Object%20Reference) (InstigatedBy :type Controller%20Object%20Reference) (DamageCauser :type Actor%20Object%20Reference))
  ;[1 1 1] Manejo de daños WIP
  (if (not true) ; Está recibiendo daño en el momento?
    (Variables|Default|SetHealth (- (Variables|Default|GetHealth) Damage))
    (if (not (> (Variables|Default|GetHealth) 0.0))
      (CallFunction|IsDeadEvent))))

(event EventBeginPlay
  ;[1 1 1] INICIO DE JUEGO
  (bind _returnvalue (UserInterface|CreateWidget "/Game/Blueprints/Player/Components/bpHUD.bpHUD_C"))
  (UserInterface|Viewport|AddtoViewport _returnvalue 1)
  (Pawn|Components|CharacterMovement|SetMovementMode (Variables|Character|GetCharacterMovement) "MOVE_Falling" 0)
  (Game|SpawnActorfromClass "/Game/Blueprints/Actors_FX/bp_Dust.bp_Dust_C" (Transformation|GetWorldTransform (Variables|Default|GetSphere)) "AlwaysSpawn" 0 0)
  (Utilities|FlowControl|Delay 1.0)
  (Pawn|Components|CharacterMovement|SetMovementMode (Variables|Character|GetCharacterMovement) "MOVE_Walking" 0)
  (bind _asgame_controller_bp (Utilities|Casting|CastToGameControllerBP (Game|GetGameMode)))
  (Variables|Default|SetGameControllerBP _asgame_controller_bp))

(event EventOnLanded
  (params (Hit :type Hit%20Result%20Structure%20%28by%20ref%29))
  ;[1 1 1] Movimiento/Salto
  ;;[1 1 1] Al aterrizar
  (Variables|Default|SetbLanded true)
  (Audio|PlaySound2D "/Game/Sounds/Player/Foot.Foot" 1.0 0.4 0.0 0 0)
  (CallFunction|LandFX)
  (Variables|Default|SetbInitiated true))

(event EventTick
  (params (DeltaSeconds :type Float%20%28single-precision%29))
  (bind _sprite (Variables|Default|GetSprite))
  (bind _returnvalue (Class|PaperFlipbookComponent|GetPlaybackPositioninFrames _sprite))
  ;[1 1 1] Animation Handler
  ;;[1 1 1] Rotación de animaciones
  (CallFunction|SetDir DeltaSeconds)
  (CallFunction|UpdateAnimation)
  (Math|Float|CompareFloat (.X (Math|Vector|BreakVector (Variables|/Script/Engine.MovementComponent|GetVelocity (Variables|Character|GetCharacterMovement)))) 0.0
    (:>
      (Transformation|SetRelativeRotation (Variables|Default|GetSprite) "0, 0, 0" false false))
    (:<
      (Transformation|SetRelativeRotation (Variables|Default|GetSprite) "0,180.000000, 0" false false)))
  (if (or (== _returnvalue 1) (== _returnvalue 3))
    (if (not (AI|Components|NavMovement|IsFalling (Variables|Character|GetCharacterMovement)))
      (Audio|PlaySound2D "/Game/Sounds/Player/StepsSnd.StepsSnd" 1.0 2.0 0.0 0 0))))

(event Input|ActionEvents|InputActionJump
  (params (Key :type Key%20Structure :default "None"))
  ;[1 1 1] Movimiento/Salto
  ;;[1 1 1] Saltando
  (:Pressed
    (CallFunction|JumpEvent))
  (:Released
    (Character|StopJumping)))

(event Input|AxisEvents|InputAxisRight
  (params (AxisValue :type Float%20%28single-precision%29))
  ;[1 1 1] Movimiento/Salto
  ;;[1 1 1] Movement Control
  (if (Variables|Default|GetbCanMoveRight)
    (Pawn|Input|AddMovementInput "1.000000, 0, 0" AxisValue false)))

(event Input|AxisEvents|InputAxisMoveUp
  (params (AxisValue :type Float%20%28single-precision%29))
  ;[1 1 1] Movimiento/Salto
  ;;[1 1 1] Escalar (escaleras)
  (if (Variables|Default|GetbCanClimb)
    (if (Math|Float|InRange(Float) AxisValue -0.1 0.1)
      (Components|Timeline|SetPlayRate (Variables|Default|GetSprite) 1.0)
      (else
        (Variables|Default|SetbIsClimbing true)
        (Variables|Default|SetbCanMoveRight true)
        (Components|Timeline|SetPlayRate (Variables|Default|GetSprite) 1.0)
        (Pawn|Components|CharacterMovement|SetMovementMode (Variables|Character|GetCharacterMovement) "MOVE_Flying" 0)
        (Pawn|Input|AddMovementInput "0, 0,1.000000" AxisValue false)))))

(fn ConstructionScript
  (Variables|/Script/Engine.CharacterMovementComponent|SetJumpZVelocity (Variables|Character|GetCharacterMovement) 3.5e+02) ; Altura del salto
  (Variables|Default|SetJumpMaxHoldTime 0.05)
  (bind _output_get (Variables|Default|SetStartScale (Transformation|GetActorScale3D)))
  (Variables|Default|SetCurrentScale _output_get)
  (Variables|Default|SetHealth (Variables|Default|GetMaxHealth)))

(fn AnimationStateMachine
  (params (bIsSlashing :type Boolean) (bIsHit :type Boolean) (bIsClimbing :type Boolean) (bIsCasting :type Boolean) (bIsAttacking2 :type Boolean) (bIsAttacking :type Boolean) (bIsDashing :type Boolean) (bIsFalling :type Boolean) (bIsMoving :type Boolean) (bIsIdleCalm :type Boolean) (bIsAlive :type Boolean))
  ;[1 1 1] Animación: Aquí van las condiciones de la animacion y el flipbook seleccionado según la animación
  (if bIsSlashing
    (LocalVariables|SetAnimationState "NewEnumerator8")
    (elif bIsHit
      (LocalVariables|SetAnimationState "NewEnumerator10")
      (elif bIsClimbing
        (LocalVariables|SetAnimationState "NewEnumerator5")
        (elif bIsCasting
          (LocalVariables|SetAnimationState "NewEnumerator7")
          (elif bIsAttacking2
            (LocalVariables|SetAnimationState "NewEnumerator11")
            (elif bIsAttacking
              (LocalVariables|SetAnimationState "NewEnumerator3")
              (elif bIsDashing
                (LocalVariables|SetAnimationState "NewEnumerator4")
                (elif bIsFalling
                  (LocalVariables|SetAnimationState "NewEnumerator2") ; salto
                  (elif bIsMoving
                    (LocalVariables|SetAnimationState "NewEnumerator1") ; movimiento
                    (elif bIsIdleCalm
                      (LocalVariables|SetAnimationState "NewEnumerator9") ; pose base
                      (elif bIsAlive
                        (LocalVariables|SetAnimationState "NewEnumerator0")
                        (else
                          (LocalVariables|SetAnimationState "NewEnumerator6") ; muerte
                          (Effects|SpawnEmitterAttached 0 0 "None" (Transformation|GetWorldLocation (Variables|Default|GetSphere)))))))))))))))
  (return (Utilities|Select :Index (LocalVariables|GetAnimationState) :NewEnumerator0 (Variables|FB|GetIdleFB) :NewEnumerator1 (Variables|FB|GetRunningFB) :NewEnumerator2 (Variables|FB|GetJumpingFB) :NewEnumerator11 (Variables|FB|GetAttack2FB) :NewEnumerator3 (Variables|FB|GetAttackFB) :NewEnumerator4 (Variables|FB|GetDashingFB) :NewEnumerator5 (Variables|FB|GetClimbingFB) :NewEnumerator6 (Variables|FB|GetDieFB) :NewEnumerator7 (Variables|FB|GetCastFB) :NewEnumerator8 (Variables|FB|GetSlashingFB) :NewEnumerator10 (Variables|FB|GetHitFB) :NewEnumerator9 (Variables|FB|GetIdleCalmFB))))

(event Custom|IsDead_Event
  (Variables|Default|SetbIsAlive false)
  (Input|DisableInput (Game|GetPlayerController 0))
  (Audio|PlaySound2D 0 1.5 0.6 0.0 0 0)
  (Pawn|Components|CharacterMovement|DisableMovement (Variables|Character|GetCharacterMovement))
  (Utilities|FlowControl|Delay 1.0)
  (Actor|DestroyActor (Game|Player|GetPlayerPawn 0)))

(event Custom|ScaleControl
  (params (bIsHealth :type Boolean))
  (if bIsHealth
    (if (not (Variables|/Game/Blueprints/GameControllerBP.GameControllerBP_C|GetbHasMushroom (Variables|Default|GetGameControllerBP)))
      (bind _scaling (Timeline|Scale Play)
        (:Update
          (Transformation|SetActorScale3D _scaling)
          (Variables|Default|SetCurrentScale (Variables|Default|GetIncreasedScale))
          (Variables|/Game/Blueprints/GameControllerBP.GameControllerBP_C|SetbHasMushroom (Variables|Default|GetGameControllerBP) true))))
    (else
      (Variables|Default|SetCurrentScale (Variables|Default|GetStartScale))
      (Transformation|SetActorScale3D (Variables|Default|GetStartScale))
      (Variables|/Game/Blueprints/GameControllerBP.GameControllerBP_C|SetbHasMushroom (Variables|Default|GetGameControllerBP) false))))