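; Coin pickup Blueprint with extra spawn behavior for coins flagged as dropped.
; On BeginPlay, a dropped coin turns off gravity on its Sphere and launches it upward at Force, with random sideways X velocity bounded by the Direction angle.
; Inner and outer collisions start query-only and switch to query-and-physics after a short delay.
; The coin then destroys itself after a further delay if its Sphere was still valid.
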(event EventBeginPlay
  (bind _force (Variables|Default|GetForce))
  (|CallParentFunction)
  (if (Variables|Default|GetbDropped)
    (Collision|SetCollisionEnabled (Variables|Default|GetInnerCollision) "QueryOnly")
    (Collision|SetCollisionEnabled (Variables|Default|GetOuterCollision) "QueryOnly")
    (Physics|SetEnableGravity (Variables|Default|GetSphere) false)
    (Class|PrimitiveComponent|SetAllPhysicsLinearVelocity (Variables|Default|GetSphere) (Math|Vector|MakeVector (* (Math|Trig|Sin(Degrees) (Math|Random|RandomFloatinRange (* (Variables|Default|GetDirection) -1.0) (Variables|Default|GetDirection))) _force) 0.0 (* (Math|Trig|Cos(Degrees) 0.0) _force)) false)
    (Utilities|FlowControl|Delay 1.0)
    (Collision|SetCollisionEnabled (Variables|Default|GetInnerCollision) "QueryAndPhysics")
    (Utilities|IsValid (Variables|Default|GetSphere)
      (:Is%20Valid
        (Collision|SetCollisionEnabled (Variables|Default|GetOuterCollision) "QueryAndPhysics")
        (Utilities|FlowControl|Delay 2.0)
        (Actor|DestroyActor)))))

(fn ConstructionScript
  (|CallParentFunction))