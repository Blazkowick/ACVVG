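; BP_PickUp_Heart is a health pickup that homes in on the player and heals on contact.
; OuterCollision caches the first overlapping bpPlayer, and Tick then lerps the ProjectileMovement velocity toward them at IncreaseSpeed.
; InnerCollision adds health and notifies GameControllerBP if the player is below full health, with no clamp on the sum.
; The heart destroys itself on player contact even when no healing occurs.
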(event OnComponentBeginOverlap(InnerCollision)
  (params (OverlappedComponent :type Primitive%20Component%20Object%20Reference) (OtherActor :type Actor%20Object%20Reference) (OtherComp :type Primitive%20Component%20Object%20Reference) (OtherBodyIndex :type Integer) (bFromSweep :type Boolean) (SweepResult :type Hit%20Result%20Structure%20%28by%20ref%29))
  (bind _asbp_player (Utilities|Casting|CastTobpPlayer OtherActor))
  (if (>= (Variables|/Game/Blueprints/Player/bpPlayer.bpPlayer_C|GetHealth _asbp_player) 1e+02)
    _
    (else
      (Variables|/Game/Blueprints/Player/bpPlayer.bpPlayer_C|SetHealth _asbp_player (+ (Variables|/Game/Blueprints/Player/bpPlayer.bpPlayer_C|GetHealth _asbp_player) 25.0))
      (Default|OnPickUp (Variables|Default|GetGameControllerBP) self)))
  (Actor|DestroyActor))

(event OnComponentBeginOverlap(OuterCollision)
  (params (OverlappedComponent :type Primitive%20Component%20Object%20Reference) (OtherActor :type Actor%20Object%20Reference) (OtherComp :type Primitive%20Component%20Object%20Reference) (OtherBodyIndex :type Integer) (bFromSweep :type Boolean) (SweepResult :type Hit%20Result%20Structure%20%28by%20ref%29))
  (bind _asbp_player (Utilities|Casting|CastTobpPlayer OtherActor))
  (Utilities|IsValid (Variables|Default|GetbpPlayer)
    (:Is%20Not%20Valid
      (Variables|Default|SetbpPlayer _asbp_player))))

(event EventTick
  (params (DeltaSeconds :type Float%20%28single-precision%29))
  (Utilities|IsValid (Variables|Default|GetbpPlayer)
    (:Is%20Valid
      (Variables|/Script/Engine.MovementComponent|SetVelocity (Variables|Default|GetProjectileMovement) (Math|Vector|Lerp(Vector) (Variables|/Script/Engine.MovementComponent|GetVelocity (Variables|Default|GetProjectileMovement)) (* (Math|Vector|Normalize (- (Transformation|GetActorLocation (Variables|Default|GetbpPlayer)) (Transformation|GetActorLocation))) (Variables|Default|GetIncreaseSpeed)) 0.1)))))

(event EventBeginPlay
  (bind _asgame_controller_bp (Utilities|Casting|CastToGameControllerBP (Game|GetGameMode)))
  (Variables|Default|SetGameControllerBP _asgame_controller_bp))

(fn ConstructionScript
  (|CallParentFunction))