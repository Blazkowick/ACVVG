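; BP_Red_Key is a red key pickup that homes in on the player once they enter its outer collision.
; That overlap caches the player, then Tick blends the projectile movement velocity toward the player's Things component, scaled by IncreaseSpeed.
; When KILL is true, it spawns a dust effect at that component and destroys itself.
; The inner overlap is empty, KILL is not set here, and the cached game controller goes unused.
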(event OnComponentBeginOverlap(InnerCollision)
  (params (OverlappedComponent :type Primitive%20Component%20Object%20Reference) (OtherActor :type Actor%20Object%20Reference) (OtherComp :type Primitive%20Component%20Object%20Reference) (OtherBodyIndex :type Integer) (bFromSweep :type Boolean) (SweepResult :type Hit%20Result%20Structure%20%28by%20ref%29)))

(event OnComponentBeginOverlap(OuterCollision)
  (params (OverlappedComponent :type Primitive%20Component%20Object%20Reference) (OtherActor :type Actor%20Object%20Reference) (OtherComp :type Primitive%20Component%20Object%20Reference) (OtherBodyIndex :type Integer) (bFromSweep :type Boolean) (SweepResult :type Hit%20Result%20Structure%20%28by%20ref%29))
  (bind _asbp_player (Utilities|Casting|CastTobpPlayer OtherActor))
  (Utilities|IsValid (Variables|Default|GetbpPlayer)
    (:Is%20Not%20Valid
      (Variables|Default|SetbpPlayer _asbp_player))))

(event Collision|EventActorBeginOverlap
  (params (OtherActor :type Actor%20Object%20Reference)))

(event EventTick
  (params (DeltaSeconds :type Float%20%28single-precision%29))
  (bind _bpplayer (Variables|Default|GetbpPlayer))
  (bind _things (Variables|/Game/Blueprints/Player/bpPlayer.bpPlayer_C|GetThings _bpplayer))
  (bind _returnvalue (Transformation|GetWorldLocation _things))
  (Utilities|IsValid (Variables|Default|GetbpPlayer)
    (:Is%20Valid
      (Variables|/Script/Engine.MovementComponent|SetVelocity (Variables|Default|GetProjectileMovement) (Math|Vector|Lerp(Vector) (Variables|/Script/Engine.MovementComponent|GetVelocity (Variables|Default|GetProjectileMovement)) (* (Math|Vector|Normalize (- _returnvalue (Transformation|GetActorLocation))) (Variables|Default|GetIncreaseSpeed)) 0.1))
      (if (Variables|Default|GetKILL)
        (Utilities|FlowControl|DoOnce false
          (:Completed
            (Game|SpawnActorfromClass "/Game/Blueprints/Actors_FX/bp_Dust.bp_Dust_C" (Math|Conversions|ToTransform(Vector) _returnvalue) "Undefined" 0 0)
            (Actor|DestroyActor)))))))

(event EventBeginPlay
  (bind _asgame_controller_bp (Utilities|Casting|CastToGameControllerBP (Game|GetGameMode)))
  (Variables|Default|SetGameControllerBP _asgame_controller_bp))

(fn ConstructionScript
  (|CallParentFunction))