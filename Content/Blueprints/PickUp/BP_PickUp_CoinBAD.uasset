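; Coin pickup Blueprint, marked as unused, that homes in on the player; no collection logic appears in this graph.
; When dropped, BeginPlay launches its gravity-free sphere at a random velocity in the XZ plane, switches both collisions from query-only to physics-enabled after a delay, then destroys it later.
; OuterCollision overlap stores the first player, and Tick lerps ProjectileMovement velocity toward them for a magnet effect.
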(event OnComponentBeginOverlap(OuterCollision)
  (params (OverlappedComponent :type Primitive%20Component%20Object%20Reference) (OtherActor :type Actor%20Object%20Reference) (OtherComp :type Primitive%20Component%20Object%20Reference) (OtherBodyIndex :type Integer) (bFromSweep :type Boolean) (SweepResult :type Hit%20Result%20Structure%20%28by%20ref%29))
  (bind _asbp_player (Utilities|Casting|CastTobpPlayer OtherActor))
  (Utilities|IsValid (Variables|Default|GetbpPlayer)
    (:Is%20Not%20Valid
      (Variables|Default|SetbpPlayer _asbp_player))))

(event EventBeginPlay
  (bind _direction (Variables|Default|GetDirection))
  (bind _direction_2 (Variables|Default|GetDirection))
  (bind _force (Variables|Default|GetForce))
  (bind _returnvalue (* _direction -1.0))
  (bind _returnvalue_2 (Math|Random|RandomFloatinRange _returnvalue _direction_2))
  ;[1 1 1] Funcion inutilizada
  (|CallParentFunction)
  (bind _asgame_controller_bp (Utilities|Casting|CastToGameControllerBP (Game|GetGameMode)))
  (Variables|Default|SetGameControllerBP _asgame_controller_bp)
  (if (Variables|Default|GetbDropped)
    (Collision|SetCollisionEnabled (Variables|Default|GetInnerCollision) "QueryOnly")
    (Collision|SetCollisionEnabled (Variables|Default|GetOuterCollision) "QueryOnly")
    (Physics|SetEnableGravity (Variables|Default|GetSphere) false)
    (Class|PrimitiveComponent|SetAllPhysicsLinearVelocity (Variables|Default|GetSphere) (Math|Vector|MakeVector (* (Math|Trig|Sin(Degrees) _returnvalue_2) _force) 0.0 (* (Math|Trig|Cos(Degrees) _returnvalue_2) _force)) false)
    (Utilities|FlowControl|Delay 1.0)
    (Collision|SetCollisionEnabled (Variables|Default|GetInnerCollision) "QueryAndPhysics")
    (Utilities|IsValid (Variables|Default|GetSphere)
      (:Is%20Valid
        (Collision|SetCollisionEnabled (Variables|Default|GetOuterCollision) "QueryAndPhysics")
        (Utilities|FlowControl|Delay 2.0)
        (Actor|DestroyActor)))))

(event EventTick
  (params (DeltaSeconds :type Float%20%28single-precision%29))
  (Utilities|IsValid (Variables|Default|GetbpPlayer)
    (:Is%20Valid
      (Variables|/Script/Engine.MovementComponent|SetVelocity (Variables|Default|GetProjectileMovement) (Math|Vector|Lerp(Vector) (Variables|/Script/Engine.MovementComponent|GetVelocity (Variables|Default|GetProjectileMovement)) (* (Math|Vector|Normalize (- (Transformation|GetActorLocation (Variables|Default|GetbpPlayer)) (Transformation|GetActorLocation))) (Variables|Default|GetIncreaseSpeed)) 0.1)))))

(fn ConstructionScript
  (|CallParentFunction))